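; Health component that tracks its owner's health and infection and sends the owner a death message when damage empties health.
; Damage and healing adjust health, while each infection hit raises infection and lowers max health by a fixed step.
; Values go as ratios to a HUD health bar fetched through the owner, with damage updating it only for BP_Player.
; The infection death check tests for zero or below, so rising infection never triggers it.
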(event Custom|TakeDamage
  (params (Damage :type Float%20%28double-precision%29))
  (if (<= (- (Variables|Default|GetCurrentHealth) Damage) 0.0)
    (Variables|Default|SetCurrentHealth 0.0)
    (Class|BPIHelperHealthComponent|OnDeath(Message) (Components|GetOwner))
    (else
      (Variables|Default|SetCurrentHealth (- (Variables|Default|GetCurrentHealth) Damage))))
  (if (.bSuccess (Utilities|Casting|CastToBP_Player (Components|GetOwner)))
    (Default|SetHealth (Variables|Default|GetHealthWidgetRef) (Math|Float|SelectFloat 0.0 (/ (Variables|Default|GetCurrentHealth) (Variables|Default|GetMaxHealth)) (<= (- (Variables|Default|GetCurrentHealth) Damage) 0.0)))))

(event Custom|TakeInfaction
  (if (<= (+ (Variables|Default|GetCurrentInfection) 1e+01) 0.0)
    (Variables|Default|SetCurrentInfection (Variables|Default|GetMaxInfection))
    (Default|SetInfection (Variables|Default|GetHealthWidgetRef) 0.0)
    (Class|BPIHelperHealthComponent|OnDeath(Message) (Components|GetOwner))
    (else
      (Variables|Default|SetCurrentInfection (+ (Variables|Default|GetCurrentInfection) 1e+01))
      (Variables|Default|SetMaxHealth (- (Variables|Default|GetMaxHealth) 1e+01))
      (Default|SetInfection (Variables|Default|GetHealthWidgetRef) (/ (Variables|Default|GetCurrentInfection) (Variables|Default|GetMaxInfection))))))

(event Custom|Heal
  (params (value :type Float%20%28double-precision%29))
  (bind _output_get (Variables|Default|SetCurrentHealth (Math|Float|Clamp(Float) (+ value (Variables|Default|GetCurrentHealth)) (Variables|Default|GetCurrentHealth) (Variables|Default|GetMaxHealth))))
  (Default|SetHealth (Variables|Default|GetHealthWidgetRef) (/ _output_get (Variables|Default|GetMaxHealth))))

(event EventBeginPlay
  (Variables|Default|SetCurrentHealth (Variables|Default|GetMaxHealth))
  (Variables|Default|SetCurrentInfection 0.0))

(event EventHealthBarWidgetRef
  (bind _player (Class|BPIHelperHealthComponent|GetRefPlayer(Message) (Components|GetOwner)))
  (bind _output_get (Variables|Default|SetHealthWidgetRef (Variables|/Game/UI/BP_PlayerHUD.BP_PlayerHUD_C|GetHealthBarWidgetRef (Variables|/Game/Blueprint/Player/BP_Player.BP_Player_C|GetPlayerHudRef _player))))
  (Default|SetHealth _output_get 1.0)
  (Default|SetInfection (Variables|Default|GetHealthWidgetRef) 0.0))

(fn GetRefPlayer
  (return 0))