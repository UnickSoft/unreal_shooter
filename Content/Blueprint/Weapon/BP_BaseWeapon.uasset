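; Base weapon for BP_Player that handles hitscan firing, ammo, reloading and HUD updates against BP_BaseZombie enemies.
; WeaponFire plays montages, spends ammo, traces and applies damage (critical on head), looping after a delay for one weapon type.
; Spread traces start at the camera, then re-trace along the muzzle when that point lies ahead of it, feeding a Niagara tracer.
; ReloadWeapon adjusts ammo counts, then re-enables firing when its montage completes.
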(event Custom|WeaponFire
  (bind _hitresult (Variables|FireWeapon|GetHitResult))
  (if (not (Variables|/Game/Blueprint/Player/BP_Player.BP_Player_C|GetIsStopFire (Variables|Default|GetRef))) :!label _label
    (Variables|FireWeapon|SetCanFire false)
    (Animation|Montage|PlayMontage (Variables|/Script/Engine.Character|GetMesh (Variables|Default|GetRef)) (Variables|FireWeapon|GetFireAnim)
      (:then
        (Animation|Montage|PlayMontage (Variables|Default|GetWeapon) (Variables|FireWeapon|GetWeaponFireAnim)
          (:then
            (CallFunction|UpdateAmmoMagazin)
            (Default|UpdateAmmoInfo (Variables|UI|GetWeaponWidgetRef) (Variables|Ammo|GetAmmoMagazin) (Variables|Ammo|GetCurrentAmmo))
            (bind _hitresult_2 (CallFunction|LineTraceLogic))
            (CallFunction|TraceEndPoint _hitresult_2)
            (CallFunction|TraceFX)
            (bind _asbp_base_zombie (Utilities|Casting|CastToBP_BaseZombie (.hitactor _hitresult))
              (:then
                (Game|Damage|ApplyDamage _asbp_base_zombie (Math|Float|SelectFloat (Variables|FireWeapon|GetCriticalDamage) (Variables|FireWeapon|GetDamage) (== (.hitbonename _hitresult) "head")) 0 self))
              (:CastFailed
                _))
            (Utilities|FlowControl|Delay (Variables|FireWeapon|GetFireRate))
            (if (Variables|Ammo|GetMagazonEmpty)
              (Variables|FireWeapon|SetCanFire false)
              (Development|PrintString "Ammo is end")
              (else
                (Variables|FireWeapon|SetCanFire true)
                (if (Utilities|Enum|Equal(Enum) (Variables|Default|GetWeaponType) "NewEnumerator1")
                  (goto _label))))))))))

(event Custom|ReloadWeapon
  (if (and (CallFunction|AmmoNotEmpty) (not (CallFunction|MagazinFull)))
    (Variables|Ammo|SetIsReload true)
    (CallFunction|CalculateAmmo)
    (Variables|Ammo|SetMagazonEmpty true)
    (Default|UpdateAmmoInfo (Variables|UI|GetWeaponWidgetRef) (Variables|Ammo|GetAmmoMagazin) (Variables|Ammo|GetCurrentAmmo))
    (Animation|Montage|PlayMontage (Variables|/Script/Engine.Character|GetMesh (Variables|Default|GetRef)) (Variables|Ammo|GetReloadAmmo)
      (:OnCompleted
        (Variables|Ammo|SetIsReload false)
        (Variables|FireWeapon|SetCanFire true)))))

(event EventBeginPlay
  (bind _asbp_player (Utilities|Casting|CastToBP_Player (Components|GetOwner)))
  (Variables|Default|SetRef _asbp_player))

(fn ConstructionScript)

(fn AttachtoHand
  (params (HandSocket :type Name))
  (Transformation|AttachComponentToComponent (Variables|/Script/Engine.Character|GetMesh (Variables|Default|GetRef)) HandSocket "SnapToTarget" "SnapToTarget" "SnapToTarget" true))

(fn SetWeaponWidgetRef
  (params (WeaponWidgetRef :type WBP%20Weapon%20Object%20Reference))
  (Variables|UI|SetWeaponWidgetRef WeaponWidgetRef))

(fn UpdateWidgetInfo
  (Default|UpdateAmmoUI (Variables|UI|GetWeaponWidgetRef) (Variables|Ammo|GetAmmoMagazin) (Variables|Ammo|GetCurrentAmmo) (Variables|UI|GetImageHUD)))

(fn UpdateAmmoMagazin
  (bind _result (Math|Integer|DecrementInt (Variables|Ammo|GetAmmoMagazin))
    (:%20%20
      (if (== _result 0)
        (Variables|Ammo|SetMagazonEmpty true)
        (else
          (Variables|Ammo|SetMagazonEmpty false))))))

(fn LineTraceLogic
  (bind _returnvalue (Game|GetPlayerController 0))
  (bind _weapon (Variables|Default|GetWeapon))
  (bind _returnvalue_2 (Transformation|GetSocketLocation _weapon "MuzzleFlash"))
  (bind (_location _rotation) (Pawn|GetPlayerViewPoint _returnvalue))
  (bind _outhit (Collision|LineTraceByChannel _location (Math|Random|RandomPointinBoundingBox (+ _location (* (Math|Rotator|GetRotationXVector _rotation) (Variables|FireWeapon|GetFireDistance))) (* "1.000000,1.000000,1.000000" (Variables|FireWeapon|GetFireSpread))) "TraceTypeQuery1" false 0 "ForDuration"))
  (Variables|FireWeapon|SetHitResult _outhit)
  (if (> (Class|KismetMathLibrary|DegAcos (Math|Vector|DotProduct (Math|Vector|GetForwardVector (Transformation|GetSocketRotation (Variables|Default|GetWeapon) "MuzzleFlash")) (- (Transformation|GetSocketLocation (Variables|Default|GetWeapon) "MuzzleFlash") (Math|Vector|SelectVector (.ImpactPoint (Collision|BreakHitResult _outhit)) (.TraceEnd (Collision|BreakHitResult _outhit)) (.bBlockingHit (Collision|BreakHitResult _outhit)))))) 9e+01)
    (bind _outhit_2 (Collision|LineTraceByChannel _returnvalue_2 (Math|Random|RandomPointinBoundingBox (+ _returnvalue_2 (* (Math|Vector|GetForwardVector (Transformation|GetSocketRotation (Variables|Default|GetWeapon) "MuzzleFlash")) (Variables|FireWeapon|GetFireDistance))) (* "1.000000,1.000000,1.000000" (Variables|FireWeapon|GetFireSpread))) "TraceTypeQuery1" false 0 "None"))
    (bind _output_get (Variables|FireWeapon|SetHitResult _outhit_2))
    (return _output_get)
    (else
      (return (Variables|FireWeapon|GetHitResult)))))

(fn TraceEndPoint
  (params (HitResult :type Hit%20Result%20Structure))
  (bind (_bblockinghit _binitialoverlap _time _distance _location _impactpoint _normal _impactnormal _physmat _hitactor _hitcomponent _hitbonename _bonename _hititem _elementindex _faceindex _tracestart _traceend) (Collision|BreakHitResult HitResult))
  (if _bblockinghit
    (Variables|FireWeapon|SetEndLineTrace _impactpoint)
    (else
      (Variables|FireWeapon|SetEndLineTrace _traceend))))

(fn TraceFX
  (bind _returnvalue (Niagara|SpawnSystematLocation (Variables|Default|GetTraceFXSystem) (Transformation|GetSocketLocation (Variables|Default|GetWeapon) "MuzzleFlash")))
  (Niagara|SetNiagaraVariable(Vector3) _returnvalue "TraceTarget" (Variables|FireWeapon|GetEndLineTrace)))

(fn AmmoNotEmpty
  (return (> (Variables|Ammo|GetCurrentAmmo) 0)))

(fn MagazinFull
  (return (== (Variables|Ammo|GetAmmoMagazin) (Variables|Ammo|GetMaxMagainAmmo))))

(fn CalculateAmmo
  (if (< (Variables|Ammo|GetCurrentAmmo) (- (Variables|Ammo|GetMaxMagainAmmo) (Variables|Ammo|GetAmmoMagazin)))
    (Variables|Ammo|SetAmmoMagazin (+ (Variables|Ammo|GetAmmoMagazin) (Variables|Ammo|GetCurrentAmmo)))
    (Variables|Ammo|SetCurrentAmmo 0)
    (else
      (bind _output_get (LocalVariables|SetCurrentAddAmmo (- (Variables|Ammo|GetMaxMagainAmmo) (Variables|Ammo|GetAmmoMagazin))))
      (Variables|Ammo|SetCurrentAmmo (- (Variables|Ammo|GetCurrentAmmo) _output_get)))))